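; BP_TrackerBot is a tracker bot actor that queries a navigation path to the first player pawn and scales its audio with speed.
; On BeginPlay the authority runs one synchronous pathfind from the bot's location, but the loop over path points is empty and its debug sphere draw is disconnected.
; Each Tick maps velocity magnitude to the Audio component's volume multiplier, so faster movement sounds louder.
; The graph contains no movement logic.
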(event Custom|FindNextPathPoint
  (if (Ability|HasAuthority)
    (bind _returnvalue (Class|NavigationSystemV1|FindPathtoActorSynchronously (Transformation|GetActorLocation) (Game|Player|GetPlayerPawn 0) 5e+01 0 0))
    (for _array_element (Variables|/Script/NavigationSystem.NavigationPath|GetPathPoints _returnvalue)
      _)))

(event EventTick
  (params (DeltaSeconds :type Float%20%28single-precision%29))
  (bind _audio (Variables|Default|GetAudio))
  (Utilities|IsValid _audio
    (:Is%20Valid
      (Audio|Components|Audio|SetVolumeMultiplier _audio (Math|Float|MapRangeClamped (Math|Vector|VectorLength (Transformation|GetVelocity)) 5.0 7e+02 0.0 3.0) :!class /Script/Engine.AudioComponent))))

(event EventBeginPlay
  (CallFunction|FindNextPathPoint))

(fn ConstructionScript)