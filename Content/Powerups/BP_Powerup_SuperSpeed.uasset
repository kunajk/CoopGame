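; Super speed powerup that temporarily doubles the walk speed of the actor it is activated for.
; OnActivated stores that actor as User, caches its CharacterMovementComponent MaxWalkSpeed, then sets the doubled value.
; OnExpired restores the cached speed if User is still valid.
; The Blueprint only reacts to these two events and contains no timing or pickup logic of its own.
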(event EventBeginPlay)

(event Collision|EventActorBeginOverlap
  (params (OtherActor :type Actor%20Object%20Reference)))

(event EventTick
  (params (DeltaSeconds :type Float%20%28single-precision%29)))

(event EventOnActivated
  (params (ActivatedFor :type Actor%20Object%20Reference))
  (bind _returnvalue (Actor|GetComponentbyClass ActivatedFor "/Script/Engine.CharacterMovementComponent"))
  (Variables|Default|SetUser ActivatedFor)
  (bind _output_get (Variables|Default|SetSavedMaxSpeed (Variables|/Script/Engine.CharacterMovementComponent|GetMaxWalkSpeed _returnvalue)))
  (Variables|/Script/Engine.CharacterMovementComponent|SetMaxWalkSpeed _returnvalue (* _output_get 2.0)))

(event EventOnExpired
  (Utilities|IsValid (Variables|Default|GetUser)
    (:Is%20Valid
      (Variables|/Script/Engine.CharacterMovementComponent|SetMaxWalkSpeed (Actor|GetComponentbyClass (Variables|Default|GetUser) "/Script/Engine.CharacterMovementComponent") (Variables|Default|GetSavedMaxSpeed)))))

(fn ConstructionScript)